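; Radio Blueprint that lets the player cycle through three music stations with NextRadio and PrevRadio input actions.
; BeginPlay fills a list with the Airpop, SynthFM and 66Sorrock audio sources and selects the first.
; Next and previous wrap around the list.
; SetRadio crossfades linearly, raising the selected station and lowering the others to near silence with AdjustVolume rather than stopping them.
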(event `self.ReceiveBeginPlay`
  (bind _radiolist (`self.RadioList`))
  (`KismetArrayLibrary.Array_Add` _radiolist (`self.Airpop`))
  (`KismetArrayLibrary.Array_Add` _radiolist (`self.SynthFM`))
  (`KismetArrayLibrary.Array_Add` _radiolist (`self.66Sorrock`))
  (`self.SetRadio` 0))

(event `self.ReceiveTick`
  (params (DeltaSeconds :type "Float (single-precision)")))

(event `InputAction|NextRadio`
  (params (Key :type "Key Structure"))
  (:`Pressed`
    (`self.NextRadio`)))

(event `InputAction|PrevRadio`
  (params (Key :type "Key Structure"))
  (:`Pressed`
    (`self.PrevRadio`)))

(fn `NextRadio`
  (bind _returnvalue (+ (`self.SelectedRadio`) 1))
  (if (>= _returnvalue (`KismetArrayLibrary.Array_Length` (`self.RadioList`)))
    (`self.SetRadio` 0)
    (else
      (`self.SetRadio` _returnvalue))))

(fn `PrevRadio`
  (bind _returnvalue (- (`self.SelectedRadio`) 1))
  (if (< _returnvalue 0)
    (`self.SetRadio` (- (`KismetArrayLibrary.Array_Length` (`self.RadioList`)) 1))
    (else
      (`self.SetRadio` _returnvalue))))

(fn `UserConstructionScript`)