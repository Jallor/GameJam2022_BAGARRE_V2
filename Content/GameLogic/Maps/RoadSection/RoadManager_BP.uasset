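; Road manager that builds an endless road by streaming randomly chosen road sections ahead of the player's Sedan.
; BeginPlay spawns the initial run, chaining each section at the previous one's EndOfScene.
; Tick compares the car's mesh position with a checkpoint at the second section's end, masked by ForwardVector.
; Reaching it spawns a new section, destroys the oldest beyond MinNbRoadSection, and updates the checkpoint.
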(event `self.ReceiveBeginPlay`
  (bind _returnvalue (`GameplayStatics.GetActorOfClass` "/Game/GameLogic/Character/Sedan.Sedan_C"))
  (set `self.PlayerCar` _returnvalue)
  (for _ (range (+ (`self.MinNbRoadSection`) 1))
    (`self.SpawnRoadSection` false)))

(event `self.ReceiveTick`
  (params (DeltaSeconds :type "Float (single-precision)"))
  (`self.GetIfReachCheckPoint`
    (:`HasReach`
      (`self.SpawnRoadSection` false))))

(fn `UserConstructionScript`)