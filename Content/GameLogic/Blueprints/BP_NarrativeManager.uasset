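; Narrative manager that runs a timed sequence of eight binary-choice dialogues during a vehicle scene, each answer visibly changing it.
; TriggerNewChoice advances the dialogue ID, fills the player HUD from a data table row, and unlocks input after the row's delays.
; OnChooseInput locks input, then spawns or attaches props, recolors the car or swaps camera post-processing.
; Dialogue six also starts a police chase; the last spawns a roadblock, optionally with a ramp.
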(event `self.ReceiveBeginPlay`
  (bind _plaquepoint (`/Game/GameLogic/Character/Sedan.PlaquePoint` (`self.CharacterReference`)))
  (bind _hud_player (`/Game/GameLogic/Character/Sedan.HUD_Player` (`self.CharacterReference`)))
  (add `/Game/GameLogic/Character/Sedan.OnChooseInput` (`self.CharacterReference`) (delegate `OnChooseInput`))
  ;[1 1 1] Intro
  (`KismetSystemLibrary.Delay` 3.0)
  (`UserWidget.PlayAnimation` _hud_player (`/Game/GameLogic/UI/HUD_Character.BlackScreen_fadeout` _hud_player) 0.0 1 "Forward" 1.0 false)
  (`self.TriggerNewChoice`)
  ;[1 1 1] spawn plaque
  (bind _returnvalue (`|SpawnActorFromClass` "/Game/GameLogic/Props/BP_Plaque.BP_Plaque_C" (`KismetMathLibrary.Conv_VectorToTransform` (`SceneComponent.K2_GetComponentLocation` _plaquepoint)) "Undefined" "OverrideRootScale" null null))
  (bind _output_get (set `self.PlaqueRef` _returnvalue))
  (`self.K2_AttachToComponent` _output_get _plaquepoint "None" "SnapToTarget" "KeepWorld" "KeepWorld" true))

(event `OnChooseInput`
  (params (Type :type String))
  (bind _spawnpoint_object (`/Game/GameLogic/Character/Sedan.SpawnPoint_Object` (`self.CharacterReference`)))
  (bind _spawnpoint_companion (`/Game/GameLogic/Character/Sedan.SpawnPoint_Companion` (`self.CharacterReference`)))
  (bind _spawnpoint_companion_2 (`/Game/GameLogic/Character/Sedan.SpawnPoint_Companion` (`self.CharacterReference`)))
  (bind _chasepoint (`/Game/GameLogic/Character/Sedan.ChasePoint` (`self.CharacterReference`)))
  (bind _characterpoint (`/Game/GameLogic/Character/Sedan.CharacterPoint` (`self.CharacterReference`)))
  (bind _characterpoint_2 (`/Game/GameLogic/Character/Sedan.CharacterPoint` (`self.CharacterReference`)))
  (bind _spawnpoint_object_2 (`/Game/GameLogic/Character/Sedan.SpawnPoint_Object` (`self.CharacterReference`)))
  (bind _spawnpoint_object2 (`/Game/GameLogic/Character/Sedan.SpawnPoint_Object2` (`self.CharacterReference`)))
  (bind _chasecamera (`/Game/GameLogic/Character/Sedan.ChaseCamera` (`self.CharacterReference`)))
  (bind _output_get (set `self.ChoiceSelection` Type))
  (if (not (`self.InputChoiceLock`))
    (`/Game/GameLogic/UI/HUD_Character.RemoveChoice` (`/Game/GameLogic/Character/Sedan.HUD_Player` (`self.CharacterReference`)) _output_get)
    (set `self.InputChoiceLock` true)
    (switch `int` (`self.CurrentDialogueID`)
      (:`1`
        (if (`KismetStringLibrary.EqualEqual_StrStr` (`self.ChoiceSelection`) "Choice1")
          ;[1 1 1] Spawn Dog
          (`KismetSystemLibrary.Delay` 0.0)
          (bind _returnvalue (`|SpawnActorFromClass` "/Game/GameLogic/Props/BP_Dog.BP_Dog_C" (`KismetMathLibrary.Conv_VectorToTransform` (`SceneComponent.K2_GetComponentLocation` _spawnpoint_object)) "Undefined" "OverrideRootScale" null null))
          (`self.K2_AttachToComponent` _returnvalue _spawnpoint_object "None" "SnapToTarget" "KeepWorld" "KeepWorld" true)
          (`self.TriggerNewChoice`)
          (else
            ;[1 1 1] Spawn Guitare
            (`KismetSystemLibrary.Delay` 0.0)
            (bind _returnvalue_2 (`|SpawnActorFromClass` "/Game/GameLogic/Props/BP_Guitare.BP_Guitare_C" (`KismetMathLibrary.Conv_VectorToTransform` (`SceneComponent.K2_GetComponentLocation` _spawnpoint_object_2)) "Undefined" "OverrideRootScale" null null))
            (`self.K2_AttachToComponent` _returnvalue_2 _spawnpoint_object_2 "None" "SnapToTarget" "KeepWorld" "KeepWorld" true)
            (`self.TriggerNewChoice`))))
      (:`2`
        (if (`KismetStringLibrary.EqualEqual_StrStr` (`self.ChoiceSelection`) "Choice1")
          ;[1 1 1] Spawn sombrero
          (bind _returnvalue_3 (`|SpawnActorFromClass` "/Game/GameLogic/Props/BP_Sombrero.BP_Sombrero_C" (`KismetMathLibrary.Conv_VectorToTransform` (`SceneComponent.K2_GetComponentLocation` _characterpoint_2)) "Undefined" "OverrideRootScale" null null))
          (`self.K2_AttachToComponent` _returnvalue_3 _characterpoint_2 "None" "SnapToTarget" "KeepWorld" "KeepWorld" true)
          (`KismetSystemLibrary.PrintString` "Spawn sombrero")
          (`self.TriggerNewChoice`)
          (else
            ;[1 1 1] Spawn strawhat
            (bind _returnvalue_4 (`|SpawnActorFromClass` "/Game/GameLogic/Props/BP_Cowboy.BP_Cowboy_C" (`KismetMathLibrary.Conv_VectorToTransform` (`SceneComponent.K2_GetComponentLocation` _characterpoint)) "Undefined" "OverrideRootScale" null null))
            (`self.K2_AttachToComponent` _returnvalue_4 _characterpoint "None" "SnapToTarget" "KeepWorld" "KeepWorld" true)
            (`KismetSystemLibrary.PrintString` "Spawn strawhat")
            (`self.TriggerNewChoice`))))
      (:`3`
        (if (`KismetStringLibrary.EqualEqual_StrStr` (`self.ChoiceSelection`) "Choice1")
          ;[1 1 1] Spawn Coyote
          (`KismetSystemLibrary.Delay` 0.0)
          (`KismetSystemLibrary.PrintString` "Spawn coyote")
          (`|SpawnActorFromClass` "/Game/GameLogic/Props/BP_Coyote.BP_Coyote_C" (`KismetMathLibrary.Conv_VectorToTransform` (`KismetMathLibrary.MakeVector` (.x (`SceneComponent.K2_GetComponentLocation` (`Actor.RootComponent` (`self.CharacterReference`)))) (+ (.y (`SceneComponent.K2_GetComponentLocation` (`Actor.RootComponent` (`self.CharacterReference`)))) -2500.0) (.z (`SceneComponent.K2_GetComponentLocation` (`Actor.RootComponent` (`self.CharacterReference`)))))) "Undefined" "OverrideRootScale" null null)
          (`self.TriggerNewChoice`)
          (else
            ;[1 1 1] Spawn Cone
            (`KismetSystemLibrary.Delay` 0.0)
            (`|SpawnActorFromClass` "/Game/GameLogic/Props/BP_Cone.BP_Cone_C" (`KismetMathLibrary.Conv_VectorToTransform` (`KismetMathLibrary.MakeVector` (.x (`SceneComponent.K2_GetComponentLocation` (`Actor.RootComponent` (`self.CharacterReference`)))) (+ (.y (`SceneComponent.K2_GetComponentLocation` (`Actor.RootComponent` (`self.CharacterReference`)))) -800.0) (.z (`SceneComponent.K2_GetComponentLocation` (`Actor.RootComponent` (`self.CharacterReference`)))))) "Undefined" "OverrideRootScale" null null)
            (`self.TriggerNewChoice`))))
      (:`4`
        (if (`KismetStringLibrary.EqualEqual_StrStr` (`self.ChoiceSelection`) "Choice1")
          ;[1 1 1] Change car to blue
          (`MeshComponent.SetScalarParameterValueOnMaterials` (`/Game/GameLogic/Character/Sedan.SM_Vehicule` (`self.CharacterReference`)) "ChangeColor" 0.5)
          (`self.TriggerNewChoice`)
          (else
            ;[1 1 1] Change car to yellow
            (`MeshComponent.SetScalarParameterValueOnMaterials` (`/Game/GameLogic/Character/Sedan.SM_Vehicule` (`self.CharacterReference`)) "ChangeColor" 1.0)
            (`self.TriggerNewChoice`))))
      (:`5`
        (if (`KismetStringLibrary.EqualEqual_StrStr` (`self.ChoiceSelection`) "Choice1")
          ;[1 1 1] Screen FX smoke
          (`CameraComponent.SetFieldOfView` _chasecamera 110.0)
          (set `CameraComponent.PostProcessSettings` (`self.CokeFX`) _chasecamera)
          (`self.TriggerNewChoice`)
          (else
            ;[1 1 1] Screen FX alcool
            (set `CameraComponent.PostProcessSettings` (`self.AlcoolFX`) (`/Game/GameLogic/Character/Sedan.ChaseCamera` (`self.CharacterReference`)))
            (`self.TriggerNewChoice`))))
      (:`6`
        (if (`KismetStringLibrary.EqualEqual_StrStr` (`self.ChoiceSelection`) "Choice1")
          ;[1 1 1] Pick the clown
          (`KismetSystemLibrary.PrintString` "Pick the clown")
          (`KismetSystemLibrary.Delay` 1.0)
          (bind _returnvalue_5 (`|SpawnActorFromClass` "/Game/GameLogic/Props/BP_Clown.BP_Clown_C" (`KismetMathLibrary.Conv_VectorToTransform` (`SceneComponent.K2_GetComponentLocation` _spawnpoint_companion_2)) "Undefined" "OverrideRootScale" null null))
          (`self.K2_AttachToComponent` _returnvalue_5 _spawnpoint_companion_2 "None" "SnapToTarget" "KeepWorld" "KeepWorld" true)
          (`self.TriggerNewChoice`)
          (else
            ;[1 1 1] Pick the catin
            (`KismetSystemLibrary.PrintString` "Pick the catin")
            (`KismetSystemLibrary.Delay` 1.0)
            (bind _returnvalue_6 (`|SpawnActorFromClass` "/Game/GameLogic/Props/BP_Catin.BP_Catin_C" (`KismetMathLibrary.Conv_VectorToTransform` (`SceneComponent.K2_GetComponentLocation` _spawnpoint_companion)) "Undefined" "OverrideRootScale" null null))
            (`self.K2_AttachToComponent` _returnvalue_6 _spawnpoint_companion "None" "SnapToTarget" "KeepWorld" "KeepWorld" true)
            (`self.TriggerNewChoice`)))
        ;[1 1 1] Police chase
        (`KismetSystemLibrary.Delay` 6.0)
        (bind _returnvalue_7 (`|SpawnActorFromClass` "/Game/GameLogic/Props/BP_Police.BP_Police_C" (`KismetMathLibrary.Conv_VectorToTransform` (`SceneComponent.K2_GetComponentLocation` _chasepoint)) "Undefined" "OverrideRootScale" null null))
        (`self.K2_AttachToComponent` _returnvalue_7 _chasepoint "None" "SnapToTarget" "KeepRelative" "KeepRelative" true))
      (:`7`
        (if (`KismetStringLibrary.EqualEqual_StrStr` (`self.ChoiceSelection`) "Choice1")
          ;[1 1 1] Billets
          (`KismetSystemLibrary.Delay` 0.0)
          (bind _returnvalue_8 (`|SpawnActorFromClass` "/Game/GameLogic/Props/BP_Billets.BP_Billets_C" (`KismetMathLibrary.Conv_VectorToTransform` (`SceneComponent.K2_GetComponentLocation` _spawnpoint_object2)) "Undefined" "OverrideRootScale" null null))
          (`self.K2_AttachToComponent` _returnvalue_8 _spawnpoint_object2 "None" "SnapToTarget" "KeepWorld" "KeepWorld" true)
          (`self.TriggerNewChoice`)
          (else
            ;[1 1 1] Plaque
            (`self.K2_DetachFromActor` (`self.PlaqueRef`) "KeepWorld" "KeepWorld" "KeepWorld")
            (`self.TriggerNewChoice`))))
      (:`8`
        (if (not (`KismetStringLibrary.EqualEqual_StrStr` (`self.ChoiceSelection`) "Choice1"))
          ;[1 1 1] Spawn Ramp
          (`KismetSystemLibrary.Delay` 0.0)
          (`|SpawnActorFromClass` "/Game/GameLogic/Props/BP_Ramp.BP_Ramp_C" (`KismetMathLibrary.Conv_VectorToTransform` (`KismetMathLibrary.MakeVector` (.x (`SceneComponent.K2_GetComponentLocation` (`Actor.RootComponent` (`self.CharacterReference`)))) (+ (.y (`SceneComponent.K2_GetComponentLocation` (`Actor.RootComponent` (`self.CharacterReference`)))) -19000.0) (.z (`SceneComponent.K2_GetComponentLocation` (`Actor.RootComponent` (`self.CharacterReference`)))))) "Undefined" "OverrideRootScale" null null))
        ;[1 1 1] Spawn Barrage
        (`KismetSystemLibrary.Delay` 0.0)
        (`|SpawnActorFromClass` "/Game/GameLogic/Props/BP_Barrage.BP_Barrage_C" (`KismetMathLibrary.Conv_VectorToTransform` (`KismetMathLibrary.MakeVector` (.x (`SceneComponent.K2_GetComponentLocation` (`Actor.RootComponent` (`self.CharacterReference`)))) (+ (.y (`SceneComponent.K2_GetComponentLocation` (`Actor.RootComponent` (`self.CharacterReference`)))) -20000.0) (.z (`SceneComponent.K2_GetComponentLocation` (`Actor.RootComponent` (`self.CharacterReference`)))))) "Undefined" "OverrideRootScale" null null)))))

(event `TriggerNewChoice`
  (bind _output_get (set `self.CurrentDialogueID` (+ (`self.CurrentDialogueID`) 1)))
  (switch `int` _output_get
    (:`1`
      ;[1 1 1] Dialogue 1
      (`KismetSystemLibrary.Delay` 10.0)
      (`self.TriggerNarrativeBox` "Dialogue_1")
      (bind _returnvalue (`|GetDataTableRow` (`self.NarrativeDataTable`) "Dialogue_1")
        (:`then`
          (bind (_line_1 _line_2_delay _line_2 _choices_delay) (break `/Game/GameLogic/Blueprints/NarrativeEntry` _returnvalue))
          (`KismetSystemLibrary.Delay` (+ 1.0 _line_2_delay _choices_delay))
          (set `self.InputChoiceLock` false))))
    (:`2`
      ;[1 1 1] Dialogue 2
      (`KismetSystemLibrary.Delay` 10.0)
      (`self.TriggerNarrativeBox` "Dialogue_2")
      (bind _returnvalue_2 (`|GetDataTableRow` (`self.NarrativeDataTable`) "Dialogue_2")
        (:`then`
          (bind (_line_1_2 _line_2_delay_2 _line_2_2 _choices_delay_2) (break `/Game/GameLogic/Blueprints/NarrativeEntry` _returnvalue_2))
          (`KismetSystemLibrary.Delay` (+ 1.0 _line_2_delay_2 _choices_delay_2))
          (set `self.InputChoiceLock` false))))
    (:`3`
      ;[1 1 1] Dialogue 3
      (`KismetSystemLibrary.Delay` 10.0)
      (`self.TriggerNarrativeBox` "Dialogue_3")
      (bind _returnvalue_3 (`|GetDataTableRow` (`self.NarrativeDataTable`) "Dialogue_3")
        (:`then`
          (bind (_line_1_3 _line_2_delay_3 _line_2_3 _choices_delay_3) (break `/Game/GameLogic/Blueprints/NarrativeEntry` _returnvalue_3))
          (`KismetSystemLibrary.Delay` (+ 1.0 _line_2_delay_3 _choices_delay_3))
          (set `self.InputChoiceLock` false))))
    (:`4`
      ;[1 1 1] Dialogue 4
      (`KismetSystemLibrary.Delay` 10.0)
      (`self.TriggerNarrativeBox` "Dialogue_4")
      (bind _returnvalue_4 (`|GetDataTableRow` (`self.NarrativeDataTable`) "Dialogue_4")
        (:`then`
          (bind (_line_1_4 _line_2_delay_4 _line_2_4 _choices_delay_4) (break `/Game/GameLogic/Blueprints/NarrativeEntry` _returnvalue_4))
          (`KismetSystemLibrary.Delay` (+ 1.0 _line_2_delay_4 _choices_delay_4))
          (set `self.InputChoiceLock` false))))
    (:`5`
      ;[1 1 1] Dialogue 5
      (`KismetSystemLibrary.Delay` 10.0)
      (`self.TriggerNarrativeBox` "Dialogue_5")
      (bind _returnvalue_5 (`|GetDataTableRow` (`self.NarrativeDataTable`) "Dialogue_5")
        (:`then`
          (bind (_line_1_5 _line_2_delay_5 _line_2_5 _choices_delay_5) (break `/Game/GameLogic/Blueprints/NarrativeEntry` _returnvalue_5))
          (`KismetSystemLibrary.Delay` (+ 1.0 _line_2_delay_5 _choices_delay_5))
          (set `self.InputChoiceLock` false))))
    (:`6`
      ;[1 1 1] Dialogue 6
      (`KismetSystemLibrary.Delay` 10.0)
      (`self.TriggerNarrativeBox` "Dialogue_6")
      (bind _returnvalue_6 (`|GetDataTableRow` (`self.NarrativeDataTable`) "Dialogue_6")
        (:`then`
          (bind (_line_1_6 _line_2_delay_6 _line_2_6 _choices_delay_6) (break `/Game/GameLogic/Blueprints/NarrativeEntry` _returnvalue_6))
          (`KismetSystemLibrary.Delay` (+ 1.0 _line_2_delay_6 _choices_delay_6))
          (set `self.InputChoiceLock` false))))
    (:`7`
      ;[1 1 1] Dialogue 7
      (`KismetSystemLibrary.Delay` 10.0)
      (`self.TriggerNarrativeBox` "Dialogue_7")
      (bind _returnvalue_7 (`|GetDataTableRow` (`self.NarrativeDataTable`) "Dialogue_7")
        (:`then`
          (bind (_line_1_7 _line_2_delay_7 _line_2_7 _choices_delay_7) (break `/Game/GameLogic/Blueprints/NarrativeEntry` _returnvalue_7))
          (`KismetSystemLibrary.Delay` (+ 1.0 _line_2_delay_7 _choices_delay_7))
          (set `self.InputChoiceLock` false))))
    (:`8`
      ;[1 1 1] Dialogue 8
      (`KismetSystemLibrary.Delay` 10.0)
      (`self.TriggerNarrativeBox` "Dialogue_8")
      (bind _returnvalue_8 (`|GetDataTableRow` (`self.NarrativeDataTable`) "Dialogue_8")
        (:`then`
          (bind (_line_1_8 _line_2_delay_8 _line_2_8 _choices_delay_8) (break `/Game/GameLogic/Blueprints/NarrativeEntry` _returnvalue_8))
          (`KismetSystemLibrary.Delay` (+ 1.0 _line_2_delay_8 _choices_delay_8))
          (set `self.InputChoiceLock` false))))))

(fn `TriggerNarrativeBox`
  (params (ChoiceName :type String))
  (bind _hud_player (`/Game/GameLogic/Character/Sedan.HUD_Player` (`self.CharacterReference`)))
  (bind _hud_player_2 (`/Game/GameLogic/Character/Sedan.HUD_Player` (`self.CharacterReference`)))
  (set `self.InputChoiceLock` true)
  (bind _returnvalue (`|GetDataTableRow` (`self.NarrativeDataTable`) (`KismetStringLibrary.Conv_StringToName` ChoiceName))
    (:`then`
      (`|ExecutionSequence`
        (:`then_0`
          (bind (_line_1 _line_2_delay _line_2 _choices_delay _choice_1 _choice_2) (break `/Game/GameLogic/Blueprints/NarrativeEntry` _returnvalue))
          (`MultiLineEditableTextBox.SetText` (`/Game/GameLogic/UI/HUD_Character.Line_1` _hud_player_2) _line_1))
        (:`then_1`
          (`MultiLineEditableTextBox.SetText` (`/Game/GameLogic/UI/HUD_Character.Line_2` _hud_player_2) _line_2))
        (:`then_2`
          (`TextBlock.SetText` (`/Game/GameLogic/UI/HUD_Character.Answer_1` _hud_player_2) _choice_1))
        (:`then_3`
          (`TextBlock.SetText` (`/Game/GameLogic/UI/HUD_Character.Answer_2` _hud_player_2) _choice_2))
        (:`then_4`
          (`Widget.SetVisibility` (`/Game/GameLogic/UI/HUD_Character.NarrativeBox` _hud_player) "Visible")
          (`/Game/GameLogic/UI/HUD_Character.DisplayChoice` _hud_player _line_2_delay _choices_delay))))
    (:`RowNotFound`
      (`KismetSystemLibrary.PrintString` "No row found"))))

(fn `UserConstructionScript`)